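; Arm actor that plays an animation while E is held and uses IK to pin the arm where it meets a surface.
; While the key is held, a gated Tick sphere-traces a short distance along world +Y from the IK trace end socket.
; The first hit sends its location and full IK alpha to Bones_AnimBP and pauses the mesh animation.
; Releasing E clears IK and unpauses.
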(event EventBeginPlay
  (bind _asbones_anim_bp (Utilities|Casting|CastToBones_AnimBP (Components|SkeletalMesh|GetAnimInstance (Variables|Default|GetSkeletalMesh)))
    (:then
      (Variables|Default|SetBonesAnimBP _asbones_anim_bp)
      (Input|EnableInput (Game|GetPlayerController 0)))
    (:CastFailed
      (Development|PrintString (|DebugBPInfo)))))

(event Collision|EventActorBeginOverlap
  (params (OtherActor :type Actor%20Object%20Reference)))

(event EventTick
  (params (DeltaSeconds :type Float%20%28single-precision%29))
  (bind _skeletalmesh (Variables|Default|GetSkeletalMesh))
  (bind _bonesanimbp (Variables|Default|GetBonesAnimBP))
  (bind _returnvalue (Transformation|GetSocketLocation _skeletalmesh "IKTrace_END_Socket"))
  (Utilities|FlowControl|Gate true
    (:Exit
      (bind (_outhit _returnvalue_2) (Collision|SphereTraceByChannel _returnvalue (+ _returnvalue "0.000000,10.000000, 0") 5.0 "TraceTypeQuery1" false 0 "None"))
      (if _returnvalue_2
        (|DoOnceMultiInput :!label _label
          (:A%20Out
            (Variables|/Game/IK_RND/Animations/Bones_AnimBP.Bones_AnimBP_C|SetIK_EffectorLocation _bonesanimbp (.location _outhit))
            (Variables|/Game/IK_RND/Animations/Bones_AnimBP.Bones_AnimBP_C|SetIK_Alpha _bonesanimbp 1.0)
            (Variables|/Script/Engine.SkeletalMeshComponent|SetbPauseAnims _skeletalmesh true)))
        (else
          (goto _label Reset%20In))))))

(event Input|KeyboardEvents|E
  (params (Key :type Key%20Structure))
  (bind _skeletalmesh (Variables|Default|GetSkeletalMesh))
  (bind _bonesanimbp (Variables|Default|GetBonesAnimBP))
  (bind _bonesanimbp_2 (Variables|Default|GetBonesAnimBP))
  (bind _returnvalue (Transformation|GetSocketLocation _skeletalmesh "IKTrace_END_Socket"))
  (:Pressed
    (Variables|/Game/IK_RND/Animations/Bones_AnimBP.Bones_AnimBP_C|SetPlayAnim _bonesanimbp 1.0)
    (Utilities|FlowControl|Gate true) ; enters at Open
  )
  (:Released
    (Variables|/Game/IK_RND/Animations/Bones_AnimBP.Bones_AnimBP_C|SetPlayAnim _bonesanimbp 0.0)
    (Variables|/Game/IK_RND/Animations/Bones_AnimBP.Bones_AnimBP_C|SetIK_Alpha _bonesanimbp_2 0.0)
    (Variables|/Script/Engine.SkeletalMeshComponent|SetbPauseAnims _skeletalmesh false)
    (Utilities|FlowControl|Gate true) ; enters at Close
  ))

(fn ConstructionScript)